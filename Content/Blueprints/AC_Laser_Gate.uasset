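; Laser gate hazard actor that blinks on and off and restarts the level when the player touches it.
; A looping one-second timer flips the Turn flag, swapping two Paper2D sprites and toggling the Box collision between query-only and disabled.
; Any overlap by a player-controlled pawn runs the RestartLevel console command.
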(event Custom|Event%20Fire
  (bind _papersprite (Variables|Default|GetPaperSprite))
  (bind _papersprite1 (Variables|Default|GetPaperSprite1))
  (bind _box (Variables|Default|GetBox))
  (if (Variables|Default|Getturn)
    (Rendering|Components|Sprite|SetSprite _papersprite "/Game/Assets/Textures/Ground/tileset_level_tiles_58.tileset_level_tiles_58")
    (Rendering|Components|Sprite|SetSprite _papersprite1 "/Game/Assets/Textures/Ground/tileset_level_tiles_49.tileset_level_tiles_49")
    (Collision|SetCollisionEnabled _box "NoCollision")
    (Variables|Default|Setturn false)
    (else
      (Rendering|Components|Sprite|SetSprite _papersprite "/Game/Assets/Textures/Ground/tileset_level_tiles_59.tileset_level_tiles_59")
      (Rendering|Components|Sprite|SetSprite _papersprite1 "/Game/Assets/Textures/Ground/tileset_level_tiles_50.tileset_level_tiles_50")
      (Collision|SetCollisionEnabled _box "QueryOnly")
      (Variables|Default|Setturn true))))

(event EventTick
  (params (DeltaSeconds :type Float%20%28single-precision%29)))

(event EventBeginPlay
  (Utilities|Time|SetTimerbyEvent (delegate Custom|Event%20Fire) 1.0 true))

(event Collision|EventActorBeginOverlap
  (params (OtherActor :type Actor%20Object%20Reference))
  (bind _aspawn (Utilities|Casting|CastToPawn OtherActor))
  (if (Pawn|IsPlayerControlled _aspawn)
    (Development|ExecuteConsoleCommand "RestartLevel" 0)))

(fn ConstructionScript)