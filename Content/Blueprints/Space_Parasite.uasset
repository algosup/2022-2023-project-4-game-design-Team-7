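; Space Parasite pawn that the player steers sideways and uses to take control of host creatures by bumping into them.
; Hitting a Lego or Scuzli pawn, subject to a cooldown check, destroys the parasite and has the player controller possess that pawn.
; Tick enables movement once a short downward trace, ignoring its Spawner, hits something, and also ramps global time dilation back up to normal speed.
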(event EventBeginPlay)

(event Collision|EventActorBeginOverlap
  (params (OtherActor :type Actor%20Object%20Reference)))

(event EventTick
  (params (DeltaSeconds :type Float%20%28single-precision%29)))

(event EventTick
  (params (DeltaSeconds :type Float%20%28single-precision%29))
  (bind _returnvalue (Transformation|GetActorLocation))
  (bind _returnvalue_2 (Collision|LineTraceByChannel _returnvalue (+ _returnvalue "0, 0,-100.000000") "TraceTypeQuery1" false (Utilities|Array|MakeArray (Variables|Default|Getspawner)) "None"))
  ;[1 1 1] possession
  (if _returnvalue_2
    (Variables|Default|Setspawned true))
  (Utilities|Time|SetGlobalTimeDilation (Math|Float|Min(Float) (+ (Class|GameplayStatics|GetGlobalTimeDilation) 0.1) 1.0)))

(event Collision|EventHit
  (params (MyComp :type Primitive%20Component%20Object%20Reference) (Other :type Actor%20Object%20Reference) (OtherComp :type Primitive%20Component%20Object%20Reference) (bSelfMoved :type Boolean) (HitLocation :type Vector :default "0, 0, 0") (HitNormal :type Vector :default "0, 0, 0") (NormalImpulse :type Vector :default "0, 0, 0") (Hit :type Hit%20Result%20Structure%20%28by%20ref%29))
  (bind _returnvalue (Utilities|GetClass Other))
  ;[1 1 1] possession
  (Math|Float|CompareFloat (Actor|GetGameTimeSinceCreation) 0.0
    (:>
      _)
    (:==
      _))
  (if (or (== "/Game/Blueprints/Lego.Lego_C" _returnvalue) (== _returnvalue "/Game/Blueprints/Scuzli.Scuzli_C"))
    (Math|Float|CompareFloat (Variables|Default|Getcooldown) (Utilities|Time|GetGameTimeinSeconds)
      (:==
        _)
      (:<
        _))
    (bind _aspawn (Utilities|Casting|CastToPawn Other))
    (Actor|DestroyActor)
    (Pawn|Possess (Game|GetPlayerController 0) _aspawn)
    (Variables|Default|Setcooldown (+ (Utilities|Time|GetGameTimeinSeconds) 1.0))))

(event Input|AxisEvents|InputAxisMoveRight
  (params (AxisValue :type Float%20%28single-precision%29))
  ;[1 1 1] Directional movements
  (if (Variables|Default|Getspawned)
    (Pawn|Input|AddMovementInput "1.000000,0.000000,0.000000" AxisValue false)))

(fn ConstructionScript)