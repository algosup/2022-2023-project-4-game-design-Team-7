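; BP_GameModelBase sets up the in-game UI and keeps a formatted play-time clock.
; On BeginPlay it creates the PlayingInterface widget and adds it to the viewport.
; Every Tick it splits the game time into minutes, seconds and milliseconds and stores the formatted text in the Timer string variable.
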(event EventBeginPlay
  (bind _returnvalue (UserInterface|CreateWidget "/Game/Menus/PlayingInterface.PlayingInterface_C"))
  (UserInterface|Viewport|AddtoViewport _returnvalue 0))

(event EventTick
  (params (DeltaSeconds :type Float%20%28single-precision%29))
  (bind _returnvalue (Utilities|Time|GetGameTimeinSeconds))
  (bind _returnvalue_2 (Math|Timespan|FromSeconds _returnvalue))
  (bind (_days _hours _minutes _seconds _milliseconds) (Math|Timespan|BreakTimespan _returnvalue_2))
  (Variables|Default|Settimer (Utilities|String|ToString(Text) (Utilities|Text|FormatText "{m}:{s}:{ms}" (Utilities|Text|ToText(Integer) _minutes) (Utilities|Text|ToText(Integer) _seconds) (Utilities|Text|ToText(Integer) _milliseconds false true 2)))))

(fn ConstructionScript)