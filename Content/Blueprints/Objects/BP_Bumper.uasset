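; BP_Bumper is a slime piston bumper that pushes whatever overlaps its Box1 trigger using the Velo vector.
; Characters are launched with LaunchCharacter, added to their current velocity, while other components have their physics linear velocity replaced.
; Only the non-character branch swaps the flipbook and sprite to the bump action, then after a short delay restores the flipbook and clears the sprite.
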(event OnComponentBeginOverlap(Box1)
  (params (OverlappedComponent :type Primitive%20Component%20Object%20Reference) (OtherActor :type Actor%20Object%20Reference) (OtherComp :type Primitive%20Component%20Object%20Reference) (OtherBodyIndex :type Integer) (bFromSweep :type Boolean) (SweepResult :type Hit%20Result%20Structure%20%28by%20ref%29))
  (bind _velo (Variables|Default|GetVelo))
  (bind _ascharacter (Utilities|Casting|CastToCharacter OtherActor)
    (:then
      (Character|LaunchCharacter _ascharacter _velo false false))
    (:CastFailed
      (Physics|SetPhysicsLinearVelocity OtherComp _velo false "None")
      (Sprite|SetFlipbook (Variables|Default|GetPaperFlipbook) "/Game/Assets/Sprites/other/Bumper/slime_piston_BumperAction.slime_piston_BumperAction")
      (Rendering|Components|Sprite|SetSprite (Variables|Default|GetPaperSprite) "/Game/Assets/Sprites/other/Bumper/slime_piston_Bumper_36.slime_piston_Bumper_36")
      (Utilities|FlowControl|Delay 0.2)
      (Sprite|SetFlipbook (Variables|Default|GetPaperFlipbook) "/Game/Assets/Sprites/other/Bumper/slime_piston_Bumper.slime_piston_Bumper")
      (Rendering|Components|Sprite|SetSprite (Variables|Default|GetPaperSprite) 0))))

(fn ConstructionScript)