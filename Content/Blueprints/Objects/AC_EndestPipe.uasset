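; AC_EndestPipe is the end-of-game trigger that plays the outro when its Box is overlapped.
; On overlap it saves, shows an End widget with mouse-locked UI-only input, and opens the Outro source on the Intout media player.
; Two widget images appear after a short delay.
; Once the video duration plus a brief buffer elapses, it deletes the Check_p save slot and loads the LevelName level.
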(event OnComponentBeginOverlap(Box)
  (params (OverlappedComponent :type Primitive%20Component%20Object%20Reference) (OtherActor :type Actor%20Object%20Reference) (OtherComp :type Primitive%20Component%20Object%20Reference) (OtherBodyIndex :type Integer) (bFromSweep :type Boolean) (SweepResult :type Hit%20Result%20Structure%20%28by%20ref%29))
  (bind _intout (Variables|Default|Getintout))
  (Utilities|Save true)
  (bind _returnvalue (UserInterface|CreateWidget "/Game/Menus/End.End_C"))
  (UserInterface|Viewport|AddtoViewport _returnvalue 0)
  (Input|SetInputModeUIOnly (Game|GetPlayerController 0) _returnvalue "LockAlways")
  (AddComponent|AddMediaSoundComponent false)
  (Media|MediaPlayer|OpenSource _intout "/Game/Movies/outro.outro")
  (Utilities|FlowControl|Delay 0.3)
  (Widget|SetVisibility (Variables|/Game/Menus/End.End_C|GetImage_3 _returnvalue) "Visible")
  (Widget|SetVisibility (Variables|/Game/Menus/End.End_C|GetImage_111 _returnvalue) "Visible")
  (Utilities|FlowControl|Delay (Math|Conversions|ToFloat(Integer) (+ (Math|Timespan|GetSeconds (Media|MediaPlayer|GetDuration _intout)) 3)))
  (SaveGame|DeleteGameinSlot "Check_p")
  (Game|OpenLevel(byName) (Utilities|String|StringToName (Variables|Default|GetlevelName))))

(fn ConstructionScript)