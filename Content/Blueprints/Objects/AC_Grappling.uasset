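; Grappling hook projectile actor that launches toward a destination point and physically tethers itself to the actor that spawned it.
; On BeginPlay it sets its projectile velocity from the offset between its location and Dest, so launch speed scales with distance.
; A physics constraint then links the parent actor's Box component to the hook's own Cube.
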(event EventBeginPlay
  (Variables|/Script/Engine.MovementComponent|SetVelocity (Variables|Default|GetProjectileMovement) (* (- (Transformation|GetActorLocation) (Variables|Default|Getdest)) -5.0))
  (Class|PhysicsConstraintComponent|SetConstrainedComponents (Variables|Default|GetPhysicsConstraint) (Variables|/Game/Blueprints/Characters/BP_Grappler.BP_Grappler_C|GetBox (Variables|Default|Getparent_act)) "None" (Variables|Default|GetCube) "None"))

(fn ConstructionScript)