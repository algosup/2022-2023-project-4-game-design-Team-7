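; Moving platform that travels its Box component back and forth along a path of placed Endpoint actors.
; On BeginPlay it builds the waypoint list from the Box's starting world location followed by each endpoint's location.
; An endless delay-driven loop eases the Box to each waypoint with MoveComponentTo, flipping the index step at either end.
; Move duration is the waypoint's distance from the actor's location divided by Speed.
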(event EventBeginPlay
  (bind _output_get (Variables|Default|SetActual_Spawn (Utilities|Array|MakeArray (Transformation|GetWorldLocation (Variables|Default|GetBox)))))
  (for _array_element (Variables|Default|GetEndpoints)
    (Utilities|Array|AppendArray _output_get (Utilities|Array|MakeArray (Transformation|GetActorLocation _array_element))))
  (Utilities|FlowControl|RetriggerableDelay 0.0 :!label _label)
  (Math|Integer|CompareInt (Variables|Default|GetIndex%20Loop) (Utilities|Array|Length (Variables|Default|GetActual_Spawn))
    (:==
      _)
    (:<
      (Math|Integer|CompareInt (Variables|Default|GetIndex%20Loop)
        (:>
          (Components|MoveComponentTo (Variables|Default|GetBox) (Utilities|Array|Get(acopy) (Variables|Default|GetActual_Spawn) (Variables|Default|GetIndex%20Loop)) "0, 0, 0" true true (/ (Math|Vector|Distance(Vector) (Utilities|Array|Get(acopy) (Variables|Default|GetActual_Spawn) (Variables|Default|GetIndex%20Loop)) (Transformation|GetActorLocation)) (Variables|Default|Getspeed)) false :!label _label_2)
          (Variables|Default|SetIndex%20Loop (+ (Variables|Default|GetIndex%20Loop) (Variables|Default|Getretro_indexing)))
          (goto _label))
        (:==
          (goto _label_2))
        (:<
          _))))
  (bind _output_get_2 (Variables|Default|Setretro_indexing (* (Variables|Default|Getretro_indexing) -1)))
  (Variables|Default|SetIndex%20Loop (+ (Variables|Default|GetIndex%20Loop) _output_get_2))
  (goto _label))

(event Collision|EventActorBeginOverlap
  (params (OtherActor :type Actor%20Object%20Reference)))

(fn ConstructionScript)