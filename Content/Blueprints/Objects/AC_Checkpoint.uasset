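; Checkpoint actor that saves the respawn location, pawn class and current level when its box is overlapped.
; A player-controlled pawn recolors two sprites and sets the data: box X/Z with pawn Y, and its class, substituting DefaultPawn for BP_Space_Parasite.
; Sequence then writes Save_Check and Save_Level on any overlap, even non-player ones.
; Existence checks query different slot names ("check", "lv") than those saved ("Check_p", "Lv_S").
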(event OnComponentBeginOverlap(Box)
  (params (OverlappedComponent :type Primitive%20Component%20Object%20Reference) (OtherActor :type Actor%20Object%20Reference) (OtherComp :type Primitive%20Component%20Object%20Reference) (OtherBodyIndex :type Integer) (bFromSweep :type Boolean) (SweepResult :type Hit%20Result%20Structure%20%28by%20ref%29))
  (bind _returnvalue (Game|Player|GetPlayerPawn 0))
  (bind _returnvalue_2 (Transformation|GetWorldLocation OverlappedComponent))
  (bind _returnvalue_3 (Utilities|GetClass _returnvalue))
  ;[1 1 1] Save at Checkpoint
  (Utilities|FlowControl|Sequence
    (:then_0
      ;;[1 1 1] Get data to save
      (bind _aspawn (Utilities|Casting|CastToPawn OtherActor))
      (if (Pawn|IsPlayerControlled _aspawn)
        (Variables|Default|SetPlayerLocation (Math|Vector|MakeVector (.x _returnvalue_2) (.y (Transformation|GetWorldLocation (Variables|/Script/Engine.Actor|GetRootComponent OtherActor))) (.z _returnvalue_2)))
        (if (Utilities|Enum|Equal(Enum) "BP_Space_Parasite_C" (Utilities|GetClassDisplayName _returnvalue_3))
          (Variables|Default|SetPawClass (Variables|Default|GetDefaultPawn))
          (else
            (Variables|Default|SetPawClass _returnvalue_3)))
        (bind _returnvalue_4 (Game|GetCurrentLevelName true))
        (Variables|Default|SetLvName (Utilities|String|StringToName _returnvalue_4))
        (Sprite|SetSpriteColor (Variables|Default|GetPaperSprite57) "(R=0.600000,G=1.000000,B=0.600000,A=1.000000)")
        (Sprite|SetSpriteColor (Variables|Default|GetPaperSprite58))))
    (:then_1
      ;;[1 1 1] Save checkpoint
      (bind _returnvalue_5 (SaveGame|DoesSaveGameExist "check"))
      (if _returnvalue_5
        (bind _returnvalue_6 (SaveGame|LoadGamefromSlot "Check_p"))
        (bind _assave_check (Utilities|Casting|CastToSave_Check _returnvalue_6))
        (Variables|/Game/Blueprints/Save_Check.Save_Check_C|SetPlayerLocation_S _assave_check (Variables|Default|GetPlayerLocation))
        (Variables|/Game/Blueprints/Save_Check.Save_Check_C|SetAlienPawn_S _assave_check (Variables|Default|GetPawClass))
        (SaveGame|SaveGametoSlot _assave_check "Check_p")
        (else
          (bind _returnvalue_7 (SaveGame|CreateSaveGameObject "/Game/Blueprints/Save_Check.Save_Check_C"))
          (Variables|/Game/Blueprints/Save_Check.Save_Check_C|SetPlayerLocation_S _returnvalue_7 (Variables|Default|GetPlayerLocation))
          (Variables|/Game/Blueprints/Save_Check.Save_Check_C|SetAlienPawn_S _returnvalue_7 (Variables|Default|GetPawClass))
          (SaveGame|SaveGametoSlot _returnvalue_7 "Check_p"))))
    (:then_2
      ;;[1 1 1] Save Level
      (bind _returnvalue_8 (SaveGame|DoesSaveGameExist "lv"))
      (if _returnvalue_8
        (bind _returnvalue_9 (SaveGame|LoadGamefromSlot "Lv_S"))
        (bind _assave_level (Utilities|Casting|CastToSave_Level _returnvalue_9))
        (Variables|/Game/Blueprints/Save_Level.Save_Level_C|SetLevelName_S _assave_level (Variables|Default|GetLvName))
        (SaveGame|SaveGametoSlot _assave_level "Lv_S")
        (else
          (bind _returnvalue_10 (SaveGame|CreateSaveGameObject "/Game/Blueprints/Save_Level.Save_Level_C"))
          (Variables|/Game/Blueprints/Save_Level.Save_Level_C|SetLevelName_S _returnvalue_10 (Variables|Default|GetLvName))
          (SaveGame|SaveGametoSlot _returnvalue_10 "Lv_S"))))))

(event EventBeginPlay)

(event Collision|EventActorBeginOverlap
  (params (OtherActor :type Actor%20Object%20Reference)))

(event EventTick
  (params (DeltaSeconds :type Float%20%28single-precision%29)))

(fn ConstructionScript)