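; Laser gate actor that blinks on and off and restarts the level when a player-controlled pawn overlaps it.
; A looping timer flips a Turn flag, alternately clearing and assigning the laser sprites on two Paper sprite components.
; Both branches set the Box to NoCollision, so the toggle never re-enables its collision.
; Actor begin overlap runs the RestartLevel console command without checking the flag.
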(event Custom|Event%20Fire
  (bind _papersprite (Variables|Default|GetPaperSprite))
  (bind _papersprite1 (Variables|Default|GetPaperSprite1))
  (bind _box (Variables|Default|GetBox))
  (if (Variables|Default|Getturn)
    (Rendering|Components|Sprite|SetSprite _papersprite 0)
    (Rendering|Components|Sprite|SetSprite _papersprite1 0)
    (Collision|SetCollisionEnabled _box "NoCollision")
    (Variables|Default|Setturn false)
    (else
      (Rendering|Components|Sprite|SetSprite _papersprite "/Game/Assets/Sprites/other/Laser/Laser_Laser_2.Laser_Laser_2")
      (Rendering|Components|Sprite|SetSprite _papersprite1 "/Game/Assets/Sprites/other/Laser/Laser_Laser_3.Laser_Laser_3")
      (Collision|SetCollisionEnabled _box "NoCollision")
      (Variables|Default|Setturn true))))

(event EventTick
  (params (DeltaSeconds :type Float%20%28single-precision%29)))

(event EventBeginPlay
  (Utilities|Time|SetTimerbyEvent (delegate Custom|Event%20Fire) 1.5 true))

(event Collision|EventActorBeginOverlap
  (params (OtherActor :type Actor%20Object%20Reference))
  (bind _aspawn (Utilities|Casting|CastToPawn OtherActor))
  (if (Pawn|IsPlayerControlled _aspawn)
    (Development|ExecuteConsoleCommand "RestartLevel" 0)))

(fn ConstructionScript)