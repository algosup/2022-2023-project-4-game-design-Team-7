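; Blinking laser hazard actor that periodically switches itself on and off.
; A looping timer set at BeginPlay by the Delay variable toggles the Active flag, flipping the actor's visibility and the Box collision between query-only and none.
; A pawn that hits it restarts the level through a console command if player-controlled, and is destroyed otherwise.
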(event EventBeginPlay)

(event Collision|EventActorBeginOverlap
  (params (OtherActor :type Actor%20Object%20Reference)))

(event EventTick
  (params (DeltaSeconds :type Float%20%28single-precision%29)))

(event Custom|Event%20Fire
  (bind _box (Variables|Default|GetBox))
  (Rendering|SetActorHiddenInGame (Variables|Default|Getactive))
  (if (Variables|Default|Getactive)
    (Collision|SetCollisionEnabled _box "NoCollision")
    (else
      (Collision|SetCollisionEnabled _box "QueryOnly")))
  (Variables|Default|Setactive (not (Variables|Default|Getactive))))

(event EventBeginPlay
  (Utilities|Time|SetTimerbyEvent (delegate Custom|Event%20Fire) (Variables|Default|Getdelay) true))

(event Collision|EventHit
  (params (MyComp :type Primitive%20Component%20Object%20Reference) (Other :type Actor%20Object%20Reference) (OtherComp :type Primitive%20Component%20Object%20Reference) (bSelfMoved :type Boolean) (HitLocation :type Vector :default "0, 0, 0") (HitNormal :type Vector :default "0, 0, 0") (NormalImpulse :type Vector :default "0, 0, 0") (Hit :type Hit%20Result%20Structure%20%28by%20ref%29))
  (bind _aspawn (Utilities|Casting|CastToPawn Other))
  (if (Pawn|IsPlayerControlled _aspawn)
    (Development|ExecuteConsoleCommand "RestartLevel" 0)
    (else
      (Actor|DestroyActor Other))))

(fn ConstructionScript)