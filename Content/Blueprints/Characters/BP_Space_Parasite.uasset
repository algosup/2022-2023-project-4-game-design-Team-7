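; Player-controlled 2D parasite worm pawn that possesses any Pawn it hits and destroys itself, with its Spawner excluded until a cooldown time passes.
; It spins along its physics velocity until Box1 overlaps a tile map after a short grace period, then crawls with the MoveRight axis.
; BeginPlay briefly sets a custom collision channel to overlap before blocking, and Tick ramps global time dilation back up to normal.
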(event EventBeginPlay)

(event Collision|EventActorBeginOverlap
  (params (OtherActor :type Actor%20Object%20Reference)))

(event EventTick
  (params (DeltaSeconds :type Float%20%28single-precision%29)))

(event OnComponentBeginOverlap(Box1)
  (params (OverlappedComponent :type Primitive%20Component%20Object%20Reference) (OtherActor :type Actor%20Object%20Reference) (OtherComp :type Primitive%20Component%20Object%20Reference) (OtherBodyIndex :type Integer) (bFromSweep :type Boolean) (SweepResult :type Hit%20Result%20Structure%20%28by%20ref%29))
  (Math|Float|CompareFloat (Actor|GetGameTimeSinceCreation) 0.2
    (:>
      _)
    (:==
      _))
  (Utilities|Casting|CastToPaperTileMapActor OtherActor)
  (Variables|Default|Setspawned true))

(event EventTick
  (params (DeltaSeconds :type Float%20%28single-precision%29))
  ;[1 1 1] possession
  (Utilities|Time|SetGlobalTimeDilation (Math|Float|Min(Float) (+ (Class|GameplayStatics|GetGlobalTimeDilation) 0.1) 1.0)))

(event EventBeginPlay
  (bind _box (Variables|Default|GetBox))
  (Collision|SetCollisionResponsetoChannel _box "ECC_GameTraceChannel1" "ECR_Overlap")
  (Utilities|FlowControl|Delay 0.5)
  (Collision|SetCollisionResponsetoChannel _box "ECC_GameTraceChannel1" "ECR_Block"))

(event Collision|EventHit
  (params (MyComp :type Primitive%20Component%20Object%20Reference) (Other :type Actor%20Object%20Reference) (OtherComp :type Primitive%20Component%20Object%20Reference) (bSelfMoved :type Boolean) (HitLocation :type Vector :default "0, 0, 0") (HitNormal :type Vector :default "0, 0, 0") (NormalImpulse :type Vector :default "0, 0, 0") (Hit :type Hit%20Result%20Structure%20%28by%20ref%29))
  (bind _spawner (Variables|Default|Getspawner))
  (bind _returnvalue (!= _spawner Other))
  ;[1 1 1] possession
  (Utilities|Casting|CastToPawn Other)
  (if (or (and (<= (Variables|Default|Getcooldown) (Utilities|Time|GetGameTimeinSeconds)) (not _returnvalue)) _returnvalue)
    (bind _aspawn (Utilities|Casting|CastToPawn Other))
    (Actor|DestroyActor)
    (Pawn|Possess (Game|GetPlayerController 0) _aspawn)))

(event Input|AxisEvents|InputAxisMoveRight
  (params (AxisValue :type Float%20%28single-precision%29))
  (bind _sprite (Variables|Default|Getsprite))
  ;[1 1 1] Directional movements
  (if (Variables|Default|Getspawned)
    (Pawn|Input|AddMovementInput "0.400000,0.000000,0.000000" AxisValue false)
    (Math|Float|CompareFloat AxisValue 0.0
      (:>
        (Transformation|SetWorldRotation _sprite "0, 0, 0" false false)
        (Sprite|SetFlipbook _sprite "/Game/Assets/Flipbook/Parasite/Worm_Thingy_Concept_Worm_Crawl.Worm_Thingy_Concept_Worm_Crawl" :!label _label))
      (:==
        (Sprite|SetFlipbook _sprite "/Game/Assets/Flipbook/Parasite/Worm_Thingy_Concept_Worm_Idle.Worm_Thingy_Concept_Worm_Idle"))
      (:<
        (Transformation|SetWorldRotation _sprite "0.000000,180.000000,0.000000" false false)
        (goto _label)))
    (else
      (bind _returnvalue (Physics|GetPhysicsLinearVelocity (Variables|Default|GetBox) "None"))
      (Math|Float|CompareFloat (.x _returnvalue) 0.0
        (:>
          (Transformation|SetWorldRotation _sprite "0, 0, 0" false false))
        (:<
          (Transformation|SetWorldRotation _sprite "0.000000,180.000000,0.000000" false false)))
      (Sprite|SetFlipbook _sprite "/Game/Assets/Flipbook/Parasite/SpinWin_Spinning_Worm.SpinWin_Spinning_Worm"))))

(fn ConstructionScript)