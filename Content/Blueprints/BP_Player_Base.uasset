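; BP_Player_Base is a player base Blueprint that handles sideways movement and lets control jump to another character on contact.
; The MoveRight axis adds movement input along world X.
; On Hit, once half a second has passed since creation, an Arcane-class actor is possessed by the first player controller if the cooldown has expired.
; Each possession starts a two-second cooldown based on game time.
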(event EventBeginPlay)

(event Collision|EventHit
  (params (MyComp :type Primitive%20Component%20Object%20Reference) (Other :type Actor%20Object%20Reference) (OtherComp :type Primitive%20Component%20Object%20Reference) (bSelfMoved :type Boolean) (HitLocation :type Vector :default "0, 0, 0") (HitNormal :type Vector :default "0, 0, 0") (NormalImpulse :type Vector :default "0, 0, 0") (Hit :type Hit%20Result%20Structure%20%28by%20ref%29))
  ;[1 1 1] possession
  (Math|Float|CompareFloat (Actor|GetGameTimeSinceCreation) 0.5
    (:>
      (if (== "/Game/Blueprints/Arcane.Arcane_C" (Utilities|GetClass Other))
        (Math|Float|CompareFloat (Variables|Default|Getcooldown) (Utilities|Time|GetGameTimeinSeconds)
          (:==
            _)
          (:<
            _))
        (bind _asarcane (Utilities|Casting|CastToArcane Other))
        (Pawn|Possess (Game|GetPlayerController 0) _asarcane)
        (Variables|Default|Setcooldown (+ (Utilities|Time|GetGameTimeinSeconds) 2.0))))))

(event Input|AxisEvents|InputAxisMoveRight
  (params (AxisValue :type Float%20%28single-precision%29))
  ;[1 1 1] Directional movements
  (Pawn|Input|AddMovementInput "1.000000,0.000000,0.000000" AxisValue false))

(fn ConstructionScript)