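; Baril is a short-lived barrel hazard that sends characters it hits to a checkpoint.
; Its Bomb graph checks the actor's age every Tick and destroys it after five seconds.
; On Hit with a Space_Parasite or Jj, it loops over all Checkpoint actors and moves the other actor to each, leaving it at the last one found.
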(event EventBeginPlay)

(event Collision|EventActorBeginOverlap
  (params (OtherActor :type Actor%20Object%20Reference)))

(event EventTick
  (params (DeltaSeconds :type Float%20%28single-precision%29)))

(event EventTick
  (params (DeltaSeconds :type Float%20%28single-precision%29))
  (Math|Float|CompareFloat (Actor|GetGameTimeSinceCreation) 5.0
    (:>
      (Actor|DestroyActor))))

(event Collision|EventHit
  (params (MyComp :type Primitive%20Component%20Object%20Reference) (Other :type Actor%20Object%20Reference) (OtherComp :type Primitive%20Component%20Object%20Reference) (bSelfMoved :type Boolean) (HitLocation :type Vector :default "0, 0, 0") (HitNormal :type Vector :default "0, 0, 0") (NormalImpulse :type Vector :default "0, 0, 0") (Hit :type Hit%20Result%20Structure%20%28by%20ref%29))
  (bind _returnvalue (Utilities|GetClass Other))
  (if (or (== _returnvalue "/Game/Blueprints/Space_Parasite.Space_Parasite_C") (== _returnvalue "/Game/Blueprints/jj.jj_C"))
    (bind _outactors (Actor|GetAllActorsOfClass "/Game/Blueprints/Checkpoint.Checkpoint_C"))
    (for _array_element _outactors
      (Transformation|SetActorLocation Other (Transformation|GetActorLocation _array_element) false false))))

(fn ConstructionScript)