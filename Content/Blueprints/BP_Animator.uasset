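; BP_Animator populates a Paper2D level at BeginPlay, using marker tiles in the tile map to place hazards and animated props.
; It scans layer 1 of the first tile map actor for Animated_TileSet tiles and converts grid cells to world positions.
; Each tile index selects a laser variant, a scaled saw, or a BP_Animation_Base given a matching flipbook for cables, pipes and other decor.
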(event EventBeginPlay
  (bind _returnvalue (Actor|GetActorOfClass "/Script/Paper2D.PaperTileMapActor"))
  (for _index (range 0 (- (Variables|/Script/Paper2D.PaperTileLayer|GetLayerHeight (Utilities|Array|Get(acopy) (Variables|/Script/Paper2D.PaperTileMap|GetTileLayers (Variables|/Script/Paper2D.PaperTileMapComponent|GetTileMap (Variables|/Script/Paper2D.PaperTileMapActor|GetRenderComponent _returnvalue))) 1)) 1))
    (for _index_2 (range 0 (- (Variables|/Script/Paper2D.PaperTileLayer|GetLayerWidth (Utilities|Array|Get(acopy) (Variables|/Script/Paper2D.PaperTileMap|GetTileLayers (Variables|/Script/Paper2D.PaperTileMapComponent|GetTileMap (Variables|/Script/Paper2D.PaperTileMapActor|GetRenderComponent _returnvalue))) 1)) 1))
      (if (Utilities|Enum|Equal(Enum) (Utilities|GetObjectName (.tileset (Class|PaperTileMapComponent|GetTile (Variables|/Script/Paper2D.PaperTileMapActor|GetRenderComponent _returnvalue) _index_2 _index 1))) "Animated_TileSet")
        (switch int (.tileindex (Class|PaperTileMapComponent|GetTile (Variables|/Script/Paper2D.PaperTileMapActor|GetRenderComponent _returnvalue) _index_2 _index 1))
          (:0
            (Game|SpawnActorfromClass "/Game/Blueprints/Objects/AC_Laser.AC_Laser_C" (Math|Transform|MakeTransform (* (+ (Transformation|GetWorldLocation (Variables|/Script/Paper2D.PaperTileMapActor|GetRenderComponent _returnvalue)) (Math|Vector|MakeVector (Math|Conversions|ToFloat(Integer) (* -64 _index_2)) 0.0 (Math|Conversions|ToFloat(Integer) (* _index -64)))) "1.000000,-10.000000,1.000000") "0, 0, 0" "1,1,1") "Undefined" 0 2.0 0))
          (:1
            (Game|SpawnActorfromClass "/Game/Blueprints/Objects/AC_Saw.AC_Saw_C" (Math|Transform|MakeTransform (* (+ (Transformation|GetWorldLocation (Variables|/Script/Paper2D.PaperTileMapActor|GetRenderComponent _returnvalue)) (Math|Vector|MakeVector (Math|Conversions|ToFloat(Integer) (* -64 _index_2)) 0.0 (Math|Conversions|ToFloat(Integer) (* _index -64)))) "1.000000,-10.000000,1.000000") "0, 0, 0" "1,1,1") "Undefined" 0 2.0 0))
          (:2
            (Game|SpawnActorfromClass "/Game/Blueprints/Objects/AC_Saw.AC_Saw_C" (Math|Transform|MakeTransform (* (+ (Transformation|GetWorldLocation (Variables|/Script/Paper2D.PaperTileMapActor|GetRenderComponent _returnvalue)) (Math|Vector|MakeVector (Math|Conversions|ToFloat(Integer) (* -64 _index_2)) 0.0 (Math|Conversions|ToFloat(Integer) (* _index -64)))) "1.000000,-10.000000,1.000000") "0, 0, 0" "2.000000,2.000000,2.000000") "Undefined" 0 2.0 0))
          (:3
            (Game|SpawnActorfromClass "/Game/Blueprints/Objects/AC_Saw.AC_Saw_C" (Math|Transform|MakeTransform (* (+ (Transformation|GetWorldLocation (Variables|/Script/Paper2D.PaperTileMapActor|GetRenderComponent _returnvalue)) (Math|Vector|MakeVector (Math|Conversions|ToFloat(Integer) (* -64 _index_2)) 0.0 (Math|Conversions|ToFloat(Integer) (* _index -64)))) "1.000000,-10.000000,1.000000") "0, 0, 0" "3.000000,3.000000,3.000000") "Undefined" 0 2.0 0))
          (:4
            (Game|SpawnActorfromClass "/Game/Blueprints/Objects/AC_Saw.AC_Saw_C" (Math|Transform|MakeTransform (* (+ (Transformation|GetWorldLocation (Variables|/Script/Paper2D.PaperTileMapActor|GetRenderComponent _returnvalue)) (Math|Vector|MakeVector (Math|Conversions|ToFloat(Integer) (* -64 _index_2)) 0.0 (Math|Conversions|ToFloat(Integer) (* _index -64)))) "1.000000,-10.000000,1.000000") "0, 0, 0" "4.000000,4.000000,4.000000") "Undefined" 0 2.0 0))
          (:5
            (Variables|Default|Setpipe1 "/Game/Assets/Flipbook/FB_Soft_cut_cable.FB_Soft_cut_cable")
            (bind _returnvalue_2 (Game|SpawnActorfromClass "/Game/Blueprints/Objects/BP_Animation_Base.BP_Animation_Base_C" (Math|Conversions|ToTransform(Vector) (+ (Transformation|GetWorldLocation (Variables|/Script/Paper2D.PaperTileMapActor|GetRenderComponent _returnvalue)) (Math|Vector|MakeVector (Math|Conversions|ToFloat(Integer) (* -64 _index_2)) 0.0 (Math|Conversions|ToFloat(Integer) (* _index -64))))) "Undefined" 0 0 :!label _label))
            (Sprite|SetFlipbook (Variables|/Game/Blueprints/Objects/BP_Animation_Base.BP_Animation_Base_C|GetPipes_Knot _returnvalue_2) (Variables|Default|Getpipe1)))
          (:6
            (Variables|Default|Setpipe1 "/Game/Assets/Flipbook/FB_Vert_cut_cable.FB_Vert_cut_cable")
            (goto _label))
          (:7
            (Variables|Default|Setpipe1 "/Game/Assets/Flipbook/FB_Soft_cut_cable.FB_Soft_cut_cable")
            (goto _label))
          (:8
            (Variables|Default|Setpipe1 "/Game/Assets/Flipbook/FB_Super_cut_cable.FB_Super_cut_cable")
            (goto _label))
          (:9
            (Variables|Default|Setpipe1 "/Game/Assets/Flipbook/FB_Pipes.FB_Pipes")
            (goto _label))
          (:10
            (Variables|Default|Setpipe1 "/Game/Assets/Flipbook/FB_Pipes_Lever.FB_Pipes_Lever")
            (goto _label))
          (:11
            (Variables|Default|Setpipe1 "/Game/Assets/Flipbook/FB_Pipes_Turn.FB_Pipes_Turn")
            (goto _label))
          (:12
            (Variables|Default|Setpipe1 "/Game/Assets/Flipbook/Pipes_Knot.Pipes_Knot")
            (goto _label))
          (:13
            (Variables|Default|Setpipe1 "/Game/Assets/Flipbook/FB_Elec_Thing.FB_Elec_Thing")
            (goto _label))
          (:14
            (Variables|Default|Setpipe1 "/Game/Assets/Flipbook/FB_PC.FB_PC")
            (goto _label))
          (:15
            (Variables|Default|Setpipe1 "/Game/Assets/Flipbook/FB_EyeLamp.FB_EyeLamp")
            (goto _label))
          (:16
            (Game|SpawnActorfromClass "/Game/Blueprints/Objects/AC_Laser.AC_Laser_C" (Math|Transform|MakeTransform (* (+ (Transformation|GetWorldLocation (Variables|/Script/Paper2D.PaperTileMapActor|GetRenderComponent _returnvalue)) (Math|Vector|MakeVector (Math|Conversions|ToFloat(Integer) (* -64 _index_2)) 0.0 (Math|Conversions|ToFloat(Integer) (* _index -64)))) "1.000000,-10.000000,1.000000") "90.000000, 0, 0" "1,1,1") "Undefined" 0 2.0 0))
          (:17
            (Game|SpawnActorfromClass "/Game/Blueprints/Objects/AC_Laser.AC_Laser_C" (Math|Transform|MakeTransform (* (+ (Transformation|GetWorldLocation (Variables|/Script/Paper2D.PaperTileMapActor|GetRenderComponent _returnvalue)) (Math|Vector|MakeVector (Math|Conversions|ToFloat(Integer) (* -64 _index_2)) 0.0 (Math|Conversions|ToFloat(Integer) (* _index -64)))) "1.000000,-10.000000,1.000000") "0, 0, 0" "1,1,1") "Undefined" 0 0.0 0))
          (:18
            (Game|SpawnActorfromClass "/Game/Blueprints/Objects/AC_Laser.AC_Laser_C" (Math|Transform|MakeTransform (* (+ (Transformation|GetWorldLocation (Variables|/Script/Paper2D.PaperTileMapActor|GetRenderComponent _returnvalue)) (Math|Vector|MakeVector (Math|Conversions|ToFloat(Integer) (* -64 _index_2)) 0.0 (Math|Conversions|ToFloat(Integer) (* _index -64)))) "1.000000,-10.000000,1.000000") "90.000000, 0, 0" "1,1,1") "Undefined" 0 0.0 0)))))))

(fn ConstructionScript)